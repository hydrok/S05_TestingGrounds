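; Infinite terrain tile that populates itself with props, rocks and AI pawns on BeginPlay through randomized PlaceActors and PlaceAIPawns calls.
; Its barrier starts solid and red, turning green and passable only while the player overlaps LockingVolume.
; When the player enters DestroyVolume, the tile asks InfiniteTerrainGameMode to spawn a tile, then destroys itself.
; GetAttachLocation exposes the Arrow's world transform as an attach point.
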(event OnComponentBeginOverlap(LockingVolume)
  (params (OverlappedComponent :type Primitive%20Component%20Object%20Reference) (OtherActor :type Actor%20Object%20Reference) (OtherComp :type Primitive%20Component%20Object%20Reference) (OtherBodyIndex :type Integer) (bFromSweep :type Boolean) (SweepResult :type Hit%20Result%20Structure%20%28by%20ref%29))
  (bind _barrier (Variables|Default|GetBarrier))
  (if (== OtherActor (Game|GetPlayerCharacter 0))
    (Collision|SetCollisionEnabled _barrier "NoCollision")
    (Rendering|Material|SetMaterial _barrier 0 "/Game/Dynamic/Terrain/GreenBarrier.GreenBarrier")))

(event OnComponentEndOverlap(LockingVolume)
  (params (OverlappedComponent :type Primitive%20Component%20Object%20Reference) (OtherActor :type Actor%20Object%20Reference) (OtherComp :type Primitive%20Component%20Object%20Reference) (OtherBodyIndex :type Integer))
  (bind _barrier (Variables|Default|GetBarrier))
  (if (== OtherActor (Game|GetPlayerCharacter 0))
    (Collision|SetCollisionEnabled _barrier "QueryAndPhysics")
    (Rendering|Material|SetMaterial _barrier 0 "/Game/Dynamic/Terrain/RedBarrier.RedBarrier")))

(event OnComponentBeginOverlap(DestroyVolume)
  (params (OverlappedComponent :type Primitive%20Component%20Object%20Reference) (OtherActor :type Actor%20Object%20Reference) (OtherComp :type Primitive%20Component%20Object%20Reference) (OtherBodyIndex :type Integer) (bFromSweep :type Boolean) (SweepResult :type Hit%20Result%20Structure%20%28by%20ref%29))
  (if (== OtherActor (Game|GetPlayerCharacter 0))
    (bind _asinfinite_terrain_game_mode (Utilities|Casting|CastToInfiniteTerrainGameMode (Game|GetGameMode)))
    (Default|SpawnTile _asinfinite_terrain_game_mode)
    (Actor|DestroyActor)))

(event Custom|CustomEvent)

(event EventTick
  (params (DeltaSeconds :type Float%20%28single-precision%29)))

(event EventBeginPlay
  (bind _barrier (Variables|Default|GetBarrier))
  (Collision|SetCollisionEnabled _barrier "QueryAndPhysics")
  (Rendering|Material|SetMaterial _barrier 0 "/Game/Dynamic/Terrain/RedBarrier.RedBarrier")
  (Class|Tile|PlaceActors "/Game/Dynamic/Terrain/Props/Container_BP.Container_BP_C" 1 3 4e+02 1.0 1.0)
  (Class|Tile|PlaceActors "/Game/Dynamic/Terrain/Props/Box2_BP.Box2_BP_C" 2 4 1e+02 1.0 1.0)
  (Class|Tile|PlaceActors "/Game/Dynamic/Terrain/Props/Canister1_BP.Canister1_BP_C" 1 7 5e+01 1.0 1.0)
  (Class|Tile|PlaceActors "/Game/Dynamic/Terrain/Props/Rock01_High_BP.Rock01_High_BP_C" 0 4 1.5e+02 1.0 5.0)
  (Class|Tile|PlaceActors "/Game/Dynamic/Terrain/Props/Rock05_High_BP.Rock05_High_BP_C" 0 4 2.5e+02 1.0 5.0)
  (Class|Tile|PlaceActors "/Game/Dynamic/Terrain/Props/Rock17_High_BP.Rock17_High_BP_C" 0 4 2.5e+02 1.0 5.0)
  (Class|Tile|PlaceActors "/Game/Dynamic/Terrain/Props/Sack1_BP.Sack1_BP_C" 1 2 2.5e+02 1.0 1.5)
  (Class|Tile|PlaceAIPawns "/Game/Dynamic/Character/Behaviour/Character_BP.Character_BP_C" 2 4 1e+02))

(fn ConstructionScript)

(fn GetAttachLocation
  (return (Transformation|GetWorldTransform (Variables|Default|GetArrow))))