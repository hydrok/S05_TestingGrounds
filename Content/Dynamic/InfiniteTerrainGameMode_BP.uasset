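; Game mode for an infinite terrain level that builds the world from chained tiles and keeps score.
; On BeginPlay it populates a NavMeshBoundsVolume pool, then spawns an initial run of Tile_BP actors.
; Each new tile receives the shared pool and supplies its attach location as the next tile's spawn transform.
; NewTileConquered increments the score, which GetScore returns.
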(event EventBeginPlay
  (Class|InfiniteTerrainGamemode|PopulateBoundsVolumePool)
  (for _index (range 0 3)
    (CallFunction|SpawnTile)))

(fn ConstructionScript)

(fn SpawnTile
  (bind _returnvalue (Game|SpawnActorfromClass "/Game/Dynamic/Terrain/Tile_BP.Tile_BP_C" (Variables|Default|GetNextTileTransform) "Undefined" 0 0))
  (Class|Tile|SetPool _returnvalue (Variables|Default|GetNavMeshBoundsVolumePool))
  (bind _attachtransform (Default|GetAttachLocation _returnvalue))
  (Variables|Default|SetNextTileTransform _attachtransform))

(fn NewTileConquered
  (Math|Integer|IncrementInt (Variables|Default|GetScore)))

(fn GetScore
  (return (Variables|Default|GetScore)))